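; Actor that hovers a physics-driven static mesh above world-static geometry.
; Each tick it line-traces straight down from the mesh by Height and, on a hit, applies a mass-independent upward acceleration scaled by HoverPower.
; The push grows as the mesh nears the surface, clamped from zero to full power, like a damping-free spring.
; While the trace hits, the mesh also spins by a fixed per-frame increment, independent of delta time.
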(event EventBeginPlay)

(event Collision|EventActorBeginOverlap
  (params (OtherActor :type Actor%20Object%20Reference)))

(event EventTick
  (params (DeltaSeconds :type Float%20%28single-precision%29))
  (bind _staticmesh (Variables|Default|GetStaticMesh))
  (bind _returnvalue (Transformation|GetWorldLocation _staticmesh))
  (bind (_outhit _returnvalue_2) (Collision|LineTraceForObjects _returnvalue (+ _returnvalue (Math|Vector|MakeVector 0.0 0.0 (* (Variables|Default|GetHeight) -1.0))) (Utilities|Array|MakeArray "ObjectTypeQuery1") false 0 "None"))
  (if _returnvalue_2
    (Physics|AddForce (Variables|Default|GetStaticMesh) (* "0, 0,1.000000" (* (Math|Float|Clamp(Float) (/ (- (Variables|Default|GetHeight) (.Distance (Collision|BreakHitResult _outhit))) 3e+02)) (Variables|Default|GetHoverPower))) "None" true)
    (Transformation|AddRelativeRotation (Variables|Default|GetStaticMesh) "0.000000,0.500000,0.500000" false false)))

(fn ConstructionScript)