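; BasicTurret is a turret that fires a projectile at the main character when it enters the detection sphere.
; Overlap events maintain the target array, and the mesh spins on Tick while that array is empty.
; On entry the mesh rotates once using a character-to-turret look-at with yaw flipped 180 degrees, then calls TurretFire.
; TurretFire spawns one half-scale projectile at the arrow and launches it forward using Impulse as velocity.
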(event OnComponentBeginOverlap(SphereTurret)
  (params (OverlappedComponent :type Primitive%20Component%20Object%20Reference) (OtherActor :type Actor%20Object%20Reference) (OtherComp :type Primitive%20Component%20Object%20Reference) (OtherBodyIndex :type Integer) (bFromSweep :type Boolean) (SweepResult :type Hit%20Result%20Structure%20%28by%20ref%29))
  (bind _as000_main_character (Utilities|Casting|CastTo000_MainCharacter OtherActor))
  (Utilities|Array|Add (Variables|Default|GetTargetsArr) _as000_main_character)
  (Transformation|SetRelativeRotation (Variables|Default|GetSkeletalMesh) (Math|Rotator|MakeRotator (.Roll (Math|Rotator|BreakRotator (Math|Rotator|FindLookatRotation (Transformation|GetWorldLocation (Variables|/Script/Engine.Character|GetCapsuleComponent _as000_main_character)) (Transformation|GetWorldLocation (Variables|Default|GetSkeletalMesh))))) (.Pitch (Math|Rotator|BreakRotator (Math|Rotator|FindLookatRotation (Transformation|GetWorldLocation (Variables|/Script/Engine.Character|GetCapsuleComponent _as000_main_character)) (Transformation|GetWorldLocation (Variables|Default|GetSkeletalMesh))))) (+ (.Yaw (Math|Rotator|BreakRotator (Math|Rotator|FindLookatRotation (Transformation|GetWorldLocation (Variables|/Script/Engine.Character|GetCapsuleComponent _as000_main_character)) (Transformation|GetWorldLocation (Variables|Default|GetSkeletalMesh))))) 1.8e+02)) false false)
  (CallFunction|TurretFire))

(event OnComponentEndOverlap(SphereTurret)
  (params (OverlappedComponent :type Primitive%20Component%20Object%20Reference) (OtherActor :type Actor%20Object%20Reference) (OtherComp :type Primitive%20Component%20Object%20Reference) (OtherBodyIndex :type Integer))
  (bind _as000_main_character (Utilities|Casting|CastTo000_MainCharacter OtherActor))
  (Utilities|Array|RemoveItem (Variables|Default|GetTargetsArr) _as000_main_character))

(event Collision|EventActorBeginOverlap
  (params (OtherActor :type Actor%20Object%20Reference)))

(event EventBeginPlay)

(event EventTick
  (params (DeltaSeconds :type Float%20%28single-precision%29))
  (if (== (Utilities|Array|Length (Variables|Default|GetTargetsArr)) 0)
    (Transformation|AddRelativeRotation (Variables|Default|GetSkeletalMesh) "0,10.000000, 0" false false)))

(fn ConstructionScript)

(fn TurretFire
  (bind _arrow (Variables|Default|GetArrow))
  (bind _returnvalue (Transformation|GetWorldTransform _arrow))
  (bind (_location _rotation) (Math|Transform|BreakTransform _returnvalue))
  (bind _returnvalue_2 (Game|SpawnActorfromClass (Variables|Default|GetProjectale) (Math|Transform|MakeTransform _location _rotation "0.500000,0.500000,0.500000") "AlwaysSpawn" 0 0))
  (Class|PrimitiveComponent|SetAllPhysicsLinearVelocity (Variables|/Game/BluePrints/Weapons/BasicProjectale.BasicProjectale_C|GetSphere _returnvalue_2) (* (Math|Vector|GetForwardVector (Variables|Default|GetArrow)) (Variables|Default|GetImpulse)) false))