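; DamageZone is a volume actor that deals continuous damage to actors while they overlap its Box component.
; Box overlap begin and end events add and remove actors in TargetsArr, with no filtering.
; Every Tick sends each tracked actor an IMakeDamage interface message, naming the zone as damager and scaling Damage by DeltaSeconds, so Damage acts as a per-second rate.
; The misleadingly named DamagePerSecond variable only stores the frame's DeltaSeconds.
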(event OnComponentBeginOverlap(Box)
  (params (OverlappedComponent :type Primitive%20Component%20Object%20Reference) (OtherActor :type Actor%20Object%20Reference) (OtherComp :type Primitive%20Component%20Object%20Reference) (OtherBodyIndex :type Integer) (bFromSweep :type Boolean) (SweepResult :type Hit%20Result%20Structure%20%28by%20ref%29))
  (Utilities|Array|Add (Variables|Default|GetTargetsArr) OtherActor))

(event OnComponentEndOverlap(Box)
  (params (OverlappedComponent :type Primitive%20Component%20Object%20Reference) (OtherActor :type Actor%20Object%20Reference) (OtherComp :type Primitive%20Component%20Object%20Reference) (OtherBodyIndex :type Integer))
  (Utilities|Array|RemoveItem (Variables|Default|GetTargetsArr) OtherActor))

(event EventBeginPlay)

(event Collision|EventActorBeginOverlap
  (params (OtherActor :type Actor%20Object%20Reference)))

(event EventTick
  (params (DeltaSeconds :type Float%20%28single-precision%29))
  (Variables|Default|SetDamagePerSecond DeltaSeconds)
  (if (> (Utilities|Array|Length (Variables|Default|GetTargetsArr)) 0)
    (for _array_element (Variables|Default|GetTargetsArr)
      (Class|MainInterface|IMakeDamage(Message) _array_element self (* (Variables|Default|GetDamagePerSecond) (Variables|Default|GetDamage))))))

(fn ConstructionScript)