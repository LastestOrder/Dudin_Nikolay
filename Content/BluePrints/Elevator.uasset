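; Elevator actor that moves its static mesh back and forth along a spline, starting automatically on BeginPlay.
; A timeline drives the mesh's relative location from the spline position at the timeline's time value.
; When each run finishes, it waits briefly, then a Forward flag selects playing in reverse or from the start, looping endlessly.
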(event Custom|Play
  (Variables|Default|SetForward true)
  (bind _splinetime (Timeline|SplineTime PlayFromStart)
    (:Update
      (Transformation|SetRelativeLocation (Variables|Default|GetStaticMesh) (Spline|GetLocationatTime (Variables|Default|GetSpline) _splinetime "Local" false) false false))
    (:Finished
      (Utilities|FlowControl|Delay 3.0)
      (if (Variables|Default|GetForward)
        (CallFunction|Reverse)
        (else
          (CallFunction|Play))))))

(event Custom|Reverse
  (Variables|Default|SetForward false)
  (bind _splinetime (Timeline|SplineTime ReverseFromEnd)
    (:Update
      (Transformation|SetRelativeLocation (Variables|Default|GetStaticMesh) (Spline|GetLocationatTime (Variables|Default|GetSpline) _splinetime "Local" false) false false))
    (:Finished
      (Utilities|FlowControl|Delay 3.0)
      (if (Variables|Default|GetForward)
        (CallFunction|Reverse)
        (else
          (CallFunction|Play))))))

(event EventBeginPlay
  (CallFunction|Play))

(event Collision|EventActorBeginOverlap
  (params (OtherActor :type Actor%20Object%20Reference)))

(event EventTick
  (params (DeltaSeconds :type Float%20%28single-precision%29)))

(fn ConstructionScript)