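; Gate Blueprint for a double swinging door that toggles open and closed each time its Activate event fires.
; Activate plays or reverses the DoorRotation timeline based on the Opening flag, then inverts the flag.
; The timeline update yaws DoorLeft and DoorRight in opposite directions, with the right leaf offset by a half turn.
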(event EventBeginPlay)

(event Collision|EventActorBeginOverlap
  (params (OtherActor :type Actor%20Object%20Reference)))

(event EventTick
  (params (DeltaSeconds :type Float%20%28single-precision%29)))

(event EventActivate
  (Utilities|FlowControl|Sequence
    (:then_0
      (if (Variables|Default|GetOpening)
        (bind _rotation (Timeline|DoorRotation Play)
          (:Update
            (Utilities|FlowControl|Sequence
              (:then_0
                (Transformation|SetRelativeRotation (Variables|Default|GetDoorRight) (Math|Rotator|MakeRotator 0.0 0.0 (+ _rotation -1.8e+02)) false false))
              (:then_1
                (Transformation|SetRelativeRotation (Variables|Default|GetDoorLeft) (Math|Rotator|MakeRotator 0.0 0.0 (* _rotation -1.0)) false false)))))
        (else
          (Timeline|DoorRotation Reverse))))
    (:then_1
      (Variables|Default|SetOpening (not (Variables|Default|GetOpening))))))

(fn ConstructionScript)