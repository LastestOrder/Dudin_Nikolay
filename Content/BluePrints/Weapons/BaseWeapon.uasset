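; Base weapon actor that the main character can target as an item and that fires physics projectiles.
; Its sphere overlap registers the weapon as the character's ActivatingItem, clearing it on exit only if it is still this weapon.
; WeaponFire spawns the Projectale class, scaled down, at the Arrow's location and rotation, then sets its sphere's linear velocity along the arrow's forward vector times Impulse.
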(event OnComponentBeginOverlap(Sphere)
  (params (OverlappedComponent :type Primitive%20Component%20Object%20Reference) (OtherActor :type Actor%20Object%20Reference) (OtherComp :type Primitive%20Component%20Object%20Reference) (OtherBodyIndex :type Integer) (bFromSweep :type Boolean) (SweepResult :type Hit%20Result%20Structure%20%28by%20ref%29))
  (bind _as000_main_character (Utilities|Casting|CastTo000_MainCharacter OtherActor))
  (Variables|/Game/Main/Character/000_MainCharacter.000_MainCharacter_C|SetActivatingItem _as000_main_character self))

(event OnComponentEndOverlap(Sphere)
  (params (OverlappedComponent :type Primitive%20Component%20Object%20Reference) (OtherActor :type Actor%20Object%20Reference) (OtherComp :type Primitive%20Component%20Object%20Reference) (OtherBodyIndex :type Integer))
  (bind _as000_main_character (Utilities|Casting|CastTo000_MainCharacter OtherActor))
  (if (== (Variables|/Game/Main/Character/000_MainCharacter.000_MainCharacter_C|GetActivatingItem _as000_main_character) self)
    (Variables|/Game/Main/Character/000_MainCharacter.000_MainCharacter_C|SetActivatingItem _as000_main_character 0)))

(event EventBeginPlay)

(event Collision|EventActorBeginOverlap
  (params (OtherActor :type Actor%20Object%20Reference)))

(event EventTick
  (params (DeltaSeconds :type Float%20%28single-precision%29)))

(fn ConstructionScript)

(fn WeaponFire
  (bind _arrow (Variables|Default|GetArrow))
  (bind _returnvalue (Transformation|GetWorldTransform _arrow))
  (bind (_location _rotation) (Math|Transform|BreakTransform _returnvalue))
  (bind _returnvalue_2 (Game|SpawnActorfromClass (Variables|Default|GetProjectale) (Math|Transform|MakeTransform _location _rotation "0.200000,0.200000,0.200000") "AlwaysSpawn" 0 0))
  (Class|PrimitiveComponent|SetAllPhysicsLinearVelocity (Variables|/Game/BluePrints/Weapons/BasicProjectale.BasicProjectale_C|GetSphere _returnvalue_2) (* (Math|Vector|GetForwardVector (Variables|Default|GetArrow)) (Variables|Default|GetImpulse)) false))