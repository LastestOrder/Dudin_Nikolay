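; AI controller for a main-character pawn that runs a behavior tree and arms the pawn on start.
; BeginPlay gathers AI_TP waypoints, stores the pawn in the blackboard, and spawns a base weapon for it to pick up.
; A sphere overlap sets the enemy target and moves toward it.
; A self-repeating random waypoint roam exists, but its starting call and the sphere's attachment to the pawn are disconnected.
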(event OnComponentBeginOverlap(Sphere)
  (params (OverlappedComponent :type Primitive%20Component%20Object%20Reference) (OtherActor :type Actor%20Object%20Reference) (OtherComp :type Primitive%20Component%20Object%20Reference) (OtherBodyIndex :type Integer) (bFromSweep :type Boolean) (SweepResult :type Hit%20Result%20Structure%20%28by%20ref%29))
  (bind _returnvalue (Pawn|GetControlledPawn))
  (if (Utilities|IsValid _returnvalue)
    (if (!= OtherActor _returnvalue)
      (Variables|Default|SetEnemyTarget OtherActor)
      (AI|AIMoveTo _returnvalue "0, 0, 0" OtherActor 5.0 false))))

(event Custom|MoveToRandomPointr
  (bind _ai_tparr (Variables|Default|GetAI_TParr))
  (bind _returnvalue (Utilities|Array|LastIndex _ai_tparr))
  (bind _returnvalue_2 (Math|Random|RandomIntegerinRange 0 _returnvalue))
  (bind _output (Utilities|Array|Get(acopy) _ai_tparr _returnvalue_2))
  (if (not (Utilities|IsValid (Variables|Default|GetEnemyTarget)))
    (Variables|Default|SetLastTP _output)
    (AI|AIMoveTo (Pawn|GetControlledPawn) "0, 0, 0" _output 5.0 false
      (:then
        (Utilities|FlowControl|Delay (Math|Random|RandomFloatinRange 0.2 4.0))
        (CallFunction|MovetoRandomPointr)))))

(event EventBeginPlay
  (Utilities|FlowControl|Sequence
    (:then_0
      (bind _outactors (Actor|GetAllActorsOfClass "/Game/AI/AI_TP.AI_TP_C"))
      (Variables|Default|SetAI_TParr _outactors)
      (bind _as000_main_character (Utilities|Casting|CastTo000_MainCharacter (Pawn|GetControlledPawn)))
      (Variables|Default|SetMyPawn _as000_main_character))
    (:then_1
      (bind _blackboardcomponent (Class|AIController|UseBlackboard "/Game/AI/MainBB.MainBB"))
      (AI|Components|Blackboard|SetValueasObject _blackboardcomponent (Variables|Default|GetSelfPawnKeyName) (Pawn|GetControlledPawn))
      (AI|RunBehaviorTree "/Game/AI/MainBT.MainBT"))
    (:then_2
      (bind _returnvalue (Game|SpawnActorfromClass "/Game/BluePrints/Weapons/BaseWeapon.BaseWeapon_C" (Math|Transform|MakeTransform (Transformation|GetActorLocation)) "AdjustIfPossibleButAlwaysSpawn" 0 0))
      (bind _output_get (Variables|/Game/Main/Character/000_MainCharacter.000_MainCharacter_C|SetActivatingItem (Variables|Default|GetMyPawn) _returnvalue))
      (Variables|/Game/Main/Character/000_MainCharacter.000_MainCharacter_C|SetDetectedItem (Variables|Default|GetMyPawn) _output_get)
      (Default|TakeWeapon (Variables|Default|GetMyPawn)))))

(event EventTick
  (params (DeltaSeconds :type Float%20%28single-precision%29)))

(fn ConstructionScript)